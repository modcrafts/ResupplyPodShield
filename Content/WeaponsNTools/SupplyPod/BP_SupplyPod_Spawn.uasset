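; BP_SupplyPod_Spawn is a drop pod Blueprint, by name the spawn variant of the supply pod, with almost no logic of its own.
; BeginPlay, Tick, drop start, near-impact, impact and controller/character setters only forward to the parent class.
; Timeline, camera shake, welcome shouting, door push and audio, nearest-player search and replication handlers for doors, lights, sides, particles and character are empty stubs.
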(event `self.ReceiveBeginPlay`
  (`parent.ReceiveBeginPlay`))

(event `self.ReceiveTick`
  (params (DeltaSeconds :type "Float (single-precision)"))
  (`parent.ReceiveTick` DeltaSeconds))

(event `Timeline_0__FinishedFunc`)

(event `Timeline_0__UpdateFunc`)

(event `self.OnDropStarted`
  (`parent.OnDropStarted`))

(event `self.OnDroppodCloseToImpact`
  (`parent.OnDroppodCloseToImpact`))

(event `self.OnDroppodImpact`
  (`parent.OnDroppodImpact`))

(event `Test Drop Pod`)

(event `HandleWelcomeShouting`
  (params (LateJoinCharacter :type "PlayerCharacter Object Reference")))

(event `CameraShake`
  (params (Shake :type "MatineeCameraShake Class Reference") (Scale :type "Float (double-precision)") (PlaySpace :type "ECameraShakePlaySpace Enum" :default "CameraLocal") (UserPlaySpaceRot :type "Rotator Structure")))

(event `self.SetController`
  (params (Controller :type "FSDPlayerController Object Reference"))
  (`parent.SetController` Controller))

(event `self.SetCharacter`
  (params (Character :type "PlayerCharacter Object Reference"))
  (`parent.SetCharacter` Character))

(fn `DoorSlamAudio`
  (params (Prim :type "PrimitiveComponent Object Reference")))

(fn `FindNearestPlayer`
  (params (FromCharacter :type "PlayerCharacter Object Reference"))
  (returns (OutNearestPlayer :type "PlayerCharacter Object Reference"))
  (return null))

(fn `OnRep_Character`)

(fn `OnRep_LightsOff`)

(fn `OnRep_RemoveDoorsIfTheyAreNotPushed`)

(fn `OnRep_RocksParticlesDisabled`)

(fn `OnRep_SidesDestroyed`)

(fn `PushDoor`
  (params (prim :type "PrimitiveComponent Object Reference")))

(fn `UserConstructionScript`)